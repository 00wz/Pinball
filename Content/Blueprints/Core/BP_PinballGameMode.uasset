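; Game mode for a pinball game that tracks score and lives, spawns balls at the level's spawn point and shows the HUD.
; A missed ball costs a life and either respawns a ball or triggers the game-over window.
; Escape, or Space for editor testing, toggles pause through a lazily created, reused pause menu, blocked after game over.
; Both menus bind restart and exit events and show the mouse cursor.
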(event `self.ReceiveBeginPlay`
  (bind _returnvalue (`|GenericCreateObject` "/Game/Blueprints/UI/WBP_PinballHud.WBP_PinballHud_C" self))
  (bind _output_get (set `self.PinballHud` _returnvalue))
  (`UserWidget.AddToViewport` _output_get 0)
  (`self.UpdateHudScore`)
  (`self.UpdateHudHealth`)
  (bind _returnvalue_2 (`GameplayStatics.GetActorOfClass` "/Game/Blueprints/BP_SpawnBallPoint.BP_SpawnBallPoint_C"))
  (set `self.BallSpawnPoint` _returnvalue_2)
  (`self.SpawnBall`)
  (`self.EnableInput` (`GameplayStatics.GetPlayerController` 0)))

(event `Key|Escape` :paused true
  (params (Key :type "Key Structure"))
  (:`Pressed`
    (`self.TogglePause` :!label _label)))

(event `Key|SpaceBar` :paused true
  (params (Key :type "Key Structure"))
  (:`Pressed`
    (goto _label)))

(fn `AddScore`
  (params (Count :type Integer))
  (set `self.Score` (+ Count (`self.Score`)))
  (`self.UpdateHudScore`))

(fn `ExitToMenu`
  (`GameplayStatics.OpenLevelBySoftObjectPtr` "/Game/Maps/L_MainMenu.L_MainMenu"))

(fn `GameOver`
  (set `self.isGameOver` true)
  (`self.ShowGameOverMenu`))

(fn `OnMissBall`
  (`/Engine/EditorBlueprintResources/StandardMacros.DecrementInt` (`self.Health`)
    (:`  `
      (`self.UpdateHudHealth`)
      (if (> (`self.Health`) 0)
        (`self.SpawnBall`)
        (else
          (`self.GameOver`))))))

(fn `RestartLevel`
  (`GameplayStatics.OpenLevelBySoftObjectPtr` "/Game/Maps/L_Level.L_Level"))

(fn `SetActivePauseMenu`
  (params (enable :type Boolean))
  (if enable
    (`|ExecutionSequence`
      (:`then_0`
        (if (not (`KismetSystemLibrary.IsValid` (`self.PauseMenu`)))
          (bind _returnvalue (`|GenericCreateObject` "/Game/Blueprints/UI/WBP_PauseWindow.WBP_PauseWindow_C" self))
          (bind _output_get (set `self.PauseMenu` _returnvalue))
          (`Widget.SetVisibility` _output_get "Collapsed")
          (`UserWidget.AddToViewport` _output_get 0)
          (add `/Game/Blueprints/UI/WBP_PauseWindow.OnClickExit` _output_get (`|CreateDelegate` :!event `ExitToMenu`))
          (add `/Game/Blueprints/UI/WBP_PauseWindow.OnClickRestart` _output_get (`|CreateDelegate` :!event `RestartLevel`))))
      (:`then_1`
        (`Widget.SetVisibility` (`self.PauseMenu`) "Visible")
        (set `PlayerController.bShowMouseCursor` true (`GameplayStatics.GetPlayerController` 0))))
    (elif (`KismetSystemLibrary.IsValid` (`self.PauseMenu`))
      (`Widget.SetVisibility` (`self.PauseMenu`) "Collapsed")
      (set `PlayerController.bShowMouseCursor` false (`GameplayStatics.GetPlayerController` 0)))))

(fn `ShowGameOverMenu`
  (bind _returnvalue (`|GenericCreateObject` "/Game/Blueprints/UI/WBP_GameOverWindow.WBP_GameOverWindow_C" self))
  (add `/Game/Blueprints/UI/WBP_GameOverWindow.OnClickRestart` _returnvalue (`|CreateDelegate` :!event `RestartLevel`))
  (add `/Game/Blueprints/UI/WBP_GameOverWindow.OnClickExit` _returnvalue (`|CreateDelegate` :!event `ExitToMenu`))
  (`UserWidget.AddToViewport` _returnvalue 0)
  (set `PlayerController.bShowMouseCursor` true (`GameplayStatics.GetPlayerController` 0)))

(fn `SpawnBall`
  (`|SpawnActorFromClass` "/Game/Blueprints/BP_Ball.BP_Ball_C" (`self.GetTransform` (`self.BallSpawnPoint`)) "Undefined" "OverrideRootScale" null null))

(fn `TogglePause`
  (if (not (`self.isGameOver`))
    (bind _output_get (set `self.isPaused` (not (`self.isPaused`))))
    (`GameplayStatics.SetGamePaused` _output_get)
    (`self.SetActivePauseMenu` _output_get)))

(fn `UpdateHudHealth`
  (`TextBlock.SetText` (`/Game/Blueprints/UI/WBP_PinballHud.Health` (`self.PinballHud`)) (`KismetTextLibrary.Conv_IntToText` (`self.Health`))))

(fn `UpdateHudScore`
  (`TextBlock.SetText` (`/Game/Blueprints/UI/WBP_PinballHud.Score` (`self.PinballHud`)) (`KismetTextLibrary.Conv_IntToText` (`self.Score`))))

(fn `UserConstructionScript`)