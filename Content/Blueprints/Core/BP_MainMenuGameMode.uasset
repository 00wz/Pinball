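; BP_MainMenuGameMode is the main menu game mode that shows the menu UI and handles starting or quitting the game.
; On BeginPlay it creates WBP_MainMenu, binds its start and exit click events, adds it to the viewport and shows the mouse cursor.
; Its Start function opens L_Level by object reference, and its Exit function quits the game.
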(event `self.ReceiveBeginPlay`
  (bind _returnvalue (`|GenericCreateObject` "/Game/Blueprints/UI/WBP_MainMenu.WBP_MainMenu_C" self))
  (add `/Game/Blueprints/UI/WBP_MainMenu.OnClickStart` _returnvalue (`|CreateDelegate` :!event `Start`))
  (add `/Game/Blueprints/UI/WBP_MainMenu.OnClickExit` _returnvalue (`|CreateDelegate` :!event `Exit`))
  (`UserWidget.AddToViewport` _returnvalue 0)
  (set `PlayerController.bShowMouseCursor` true (`GameplayStatics.GetPlayerController` 0)))

(fn `Exit`
  (`KismetSystemLibrary.QuitGame` null "Quit"))

(fn `Start`
  (`GameplayStatics.OpenLevelBySoftObjectPtr` "/Game/Maps/L_Level.L_Level"))

(fn `UserConstructionScript`)