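; BP_Flipper is a physics-driven flipper that the player swings with horizontal mouse movement.
; Scaled MouseX input accumulates into a clamped alpha that blends between the ArrowLow and ArrowHigh orientations.
; The quaternion delta from FlipperRoot to that target, converted to a rotator and divided by frame time, sets its physics angular velocity.
; Quaternions avoid incorrect rotator differences, so the flipper tracks the target through physics.
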(event `self.ReceiveBeginPlay`
  (`self.EnableInput` (`GameplayStatics.GetPlayerController` 0)))

(event `InputAxisKey|MouseX` :consume false
  (params (AxisValue :type "Float (single-precision)"))
  (bind _output_get (set `self.Duration` (`KismetMathLibrary.FClamp` (+ (* AxisValue (`self.Sensitivity`)) (`self.Duration`)))))
  (bind (_returnvalue_roll _returnvalue_pitch _returnvalue_yaw) (`KismetMathLibrary.BreakRotator` (* (`KismetMathLibrary.Quat_Rotator` (`MyBlueprintFunctionLibrary.DeltaQuat` (`MyBlueprintFunctionLibrary.LerpQuat` (`MyBlueprintFunctionLibrary.GetRotationQuat` (`self.ArrowLow`)) (`MyBlueprintFunctionLibrary.GetRotationQuat` (`self.ArrowHigh`)) _output_get) (`MyBlueprintFunctionLibrary.GetRotationQuat` (`self.FlipperRoot`)))) (/ 1.0 (`GameplayStatics.GetWorldDeltaSeconds`)))))
  (`PrimitiveComponent.SetPhysicsAngularVelocityInDegrees` (`self.FlipperRoot`) (`KismetMathLibrary.MakeVector` (- 0.0 _returnvalue_roll) (- 0.0 _returnvalue_pitch) _returnvalue_yaw) false "None"))

(fn `UserConstructionScript`)