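; BP_Plunger is a plunger actor that the player slides along a spline with horizontal mouse movement.
; It enables input for the first player on BeginPlay and accumulates sensitivity-scaled MouseX into a clamped Duration used as spline time.
; The static mesh follows by physics velocity, computed from the gap to that spline point divided by frame delta time, rather than by setting its transform.
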(event `self.ReceiveBeginPlay`
  (`self.EnableInput` (`GameplayStatics.GetPlayerController` 0)))

(event `InputAxisKey|MouseX` :consume false
  (params (AxisValue :type "Float (single-precision)"))
  (bind _output_get (set `self.Duration` (`KismetMathLibrary.FClamp` (+ (* AxisValue (`self.Sensitivity`)) (`self.Duration`)))))
  (`PrimitiveComponent.SetPhysicsLinearVelocity` (`self.StaticMesh`) (/ (- (`SplineComponent.GetLocationAtTime` (`self.Spline`) _output_get "World" false) (`SceneComponent.K2_GetComponentLocation` (`self.StaticMesh`))) (`GameplayStatics.GetWorldDeltaSeconds`)) false "None"))

(fn `UserConstructionScript`)