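; Circular flipper actor that the player spins with horizontal mouse movement, using physics velocity.
; Scaled mouse X input accumulates into an angle around the ArrowNorm forward axis, applied to the rotation stored at BeginPlay to avoid accumulated error.
; The quaternion delta between target and current rotation becomes a rotator, is divided by frame time, and sets FlipperRoot's physics angular velocity.
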(event `self.ReceiveBeginPlay`
  (bind _flipperroot (`self.FlipperRoot`))
  (`self.EnableInput` (`GameplayStatics.GetPlayerController` 0))
  (set `self.DefaultRotation` (`MyBlueprintFunctionLibrary.GetRotationQuat` _flipperroot))
  (set `self.DefaultRootRotation` (`SceneComponent.K2_GetComponentRotation` _flipperroot)))

(event `InputAxisKey|MouseX` :consume false
  (params (AxisValue :type "Float (single-precision)"))
  (bind _output_get (set `self.Duration` (+ (* AxisValue (`self.Sensitivity`)) (`self.Duration`))))
  (bind (_returnvalue_roll _returnvalue_pitch _returnvalue_yaw) (`KismetMathLibrary.BreakRotator` (* (`KismetMathLibrary.Quat_Rotator` (`MyBlueprintFunctionLibrary.DeltaQuat` (* (`MyBlueprintFunctionLibrary.GetQuatFromAxisAngle` (`SceneComponent.GetForwardVector` (`self.ArrowNorm`)) _output_get) (`self.DefaultRotation`)) (`MyBlueprintFunctionLibrary.GetRotationQuat` (`self.FlipperRoot`)))) (/ 1.0 (`GameplayStatics.GetWorldDeltaSeconds`)))))
  (`PrimitiveComponent.SetPhysicsAngularVelocityInDegrees` (`self.FlipperRoot`) (`KismetMathLibrary.MakeVector` (- 0.0 _returnvalue_roll) (- 0.0 _returnvalue_pitch) _returnvalue_yaw) false "None"))

(fn `UserConstructionScript`)